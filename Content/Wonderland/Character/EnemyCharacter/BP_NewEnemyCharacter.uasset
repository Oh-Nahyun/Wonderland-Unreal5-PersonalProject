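; Enemy character Blueprint with a state machine (Peace, Chase, Battle, Dead) that sets walk speed per state through SetEnemyState.
; It starts in Peace, and PawnSensing switches it to Chase on seeing a pawn, which it stores as EnemyInstigator.
; OnAttackBegin and OnAttackEnd toggle the AttackCollision hit window, where overlapping actors receive point damage.
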(event `self.ReceiveBeginPlay`
  (`self.SetEnemyState` "NewEnumerator0")
  (`PrimitiveComponent.SetCollisionEnabled` (`self.AttackCollision`) "NoCollision"))

(event `self.PawnSensing.OnSeePawn`
  (params (Pawn :type "Pawn Object Reference"))
  (if (`|EnumEquality` (`self.CurrentEnemyState`) "NewEnumerator0")
    (set `self.EnemyInstigator` Pawn)
    (`self.SetEnemyState` "NewEnumerator1")))

(event `self.AttackCollision.OnComponentBeginOverlap`
  (params (OverlappedComponent :type "PrimitiveComponent Object Reference") (OtherActor :type "Actor Object Reference") (OtherComp :type "PrimitiveComponent Object Reference") (OtherBodyIndex :type Integer) (bFromSweep :type Boolean) (SweepResult :type "HitResult Structure (by ref)"))
  (`GameplayStatics.ApplyPointDamage` OtherActor 10.0 (`self.GetActorForwardVector`) SweepResult (`self.GetController`) self))

(event `OnAttackBegin`
  (`PrimitiveComponent.SetCollisionEnabled` (`self.AttackCollision`) "QueryOnly"))

(event `OnAttackEnd`
  (`PrimitiveComponent.SetCollisionEnabled` (`self.AttackCollision`) "NoCollision"))

(fn `SetEnemyState`
  (params (CurrentEnemyState :type "/Game/Wonderland/Character/EnemyCharacter/AI/BPE_EnemyState Enum" :default "NewEnumerator0"))
  (if (`|EnumInequality` (`self.CurrentEnemyState`) "NewEnumerator3")
    (bind _output_get (set `self.CurrentEnemyState` CurrentEnemyState))
    (switch `/Game/Wonderland/Character/EnemyCharacter/AI/BPE_EnemyState` _output_get
      (:`NewEnumerator0`
        (set `CharacterMovementComponent.MaxWalkSpeed` 50.0 (`self.CharacterMovement`)))
      (:`NewEnumerator1`
        (set `CharacterMovementComponent.MaxWalkSpeed` 450.0 (`self.CharacterMovement`)))
      (:`NewEnumerator2`
        (set `CharacterMovementComponent.MaxWalkSpeed` 0.0 (`self.CharacterMovement`) :!label _label))
      (:`NewEnumerator3`
        (goto _label)))))

(fn `UserConstructionScript`)