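; Ambient flying bird character that travels in a straight line and removes itself after covering a distance.
; BeginPlay switches movement to Flying at a fixed speed and derives a target from the start X plus an offset.
; Tick feeds forward movement input until within a threshold of that target, then stops and destroys the actor.
; The distance check uses only world X converted to vectors, so it assumes flight toward positive X.
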(event `self.ReceiveBeginPlay`
  (bind _returnvalue_x (`KismetMathLibrary.BreakVector` (`self.K2_GetActorLocation`)))
  (set `self.TargetLocation` (`KismetMathLibrary.Conv_DoubleToVector` (+ _returnvalue_x 30000.0)))
  (`CharacterMovementComponent.SetMovementMode` (`self.CharacterMovement`) "MOVE_Flying" 0)
  (set `CharacterMovementComponent.MaxFlySpeed` 620.0 (`self.CharacterMovement`)))

(event `self.ReceiveTick`
  (params (DeltaSeconds :type "Float (single-precision)"))
  (bind _returnvalue_x (`KismetMathLibrary.BreakVector` (`self.K2_GetActorLocation`)))
  (if (<= (`KismetMathLibrary.Vector_Distance` (`KismetMathLibrary.Conv_DoubleToVector` _returnvalue_x) (`self.TargetLocation`)) 23000.0)
    (`MovementComponent.StopMovementImmediately` (`self.CharacterMovement`))
    (`self.K2_DestroyActor`)
    (else
      (`self.AddMovementInput` (`self.GetActorForwardVector`)))))

(fn `UserConstructionScript`)