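; Guide NPC that shows an interaction prompt within a sphere trigger and walks the player through dialogue.
; BeginPlay caches dialogue and quest DataTable rows into arrays, while the overlap stores a player reference.
; Each Talk call advances one line in a reused dialogue widget, swapping the name label at a fixed index.
; When lines run out it restores the player HUD, disables talking, and shows the quest widget after the first conversation.
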(event `self.ReceiveBeginPlay`
  (`|ExecutionSequence`
    (:`then_0`
      (`KismetSystemLibrary.Delay` 0.1)
      (`SceneComponent.SetVisibility` (`self.NPC Interaction Widget`) false false))
    (:`then_1`
      (bind _outrownames (`DataTableFunctionLibrary.GetDataTableRowNames` "/Game/Wonderland/System/Dialogue/DT_Dialogue.DT_Dialogue"))
      (for _array_element _outrownames
        (bind _returnvalue (`|GetDataTableRow` "/Game/Wonderland/System/Dialogue/DT_Dialogue.DT_Dialogue" _array_element)
          (:`then`
            (`KismetArrayLibrary.Array_Add` (`self.Dialogue`) _returnvalue)))))
    (:`then_2`
      (bind _outrownames_2 (`DataTableFunctionLibrary.GetDataTableRowNames` "/Game/Wonderland/System/Quest/DT_Quest.DT_Quest"))
      (for _array_element_2 _outrownames_2
        (bind _returnvalue_2 (`|GetDataTableRow` "/Game/Wonderland/System/Quest/DT_Quest.DT_Quest" _array_element_2)
          (:`then`
            (`KismetArrayLibrary.Array_Add` (`self.Quests`) _returnvalue_2)))))))

(event `self.ReceiveTick`
  (params (DeltaSeconds :type "Float (single-precision)")))

(event `self.SphereCollision.OnComponentBeginOverlap`
  (params (OverlappedComponent :type "PrimitiveComponent Object Reference") (OtherActor :type "Actor Object Reference") (OtherComp :type "PrimitiveComponent Object Reference") (OtherBodyIndex :type Integer) (bFromSweep :type Boolean) (SweepResult :type "HitResult Structure (by ref)"))
  (`SceneComponent.SetVisibility` (`self.NPC Interaction Widget`) true false)
  (set `self.IsInSphereCollision` true)
  (bind _asbp_player_character (cast `/Game/Wonderland/Prop/Characters/PlayerCharacter/BP_PlayerCharacter` OtherActor))
  (set `self.BPPlayerCharacterRef` _asbp_player_character))

(event `self.SphereCollision.OnComponentEndOverlap`
  (params (OverlappedComponent :type "PrimitiveComponent Object Reference") (OtherActor :type "Actor Object Reference") (OtherComp :type "PrimitiveComponent Object Reference") (OtherBodyIndex :type Integer))
  (`SceneComponent.SetVisibility` (`self.NPC Interaction Widget`) false false)
  (set `self.IsInSphereCollision` false))

(event `/Game/Wonderland/System/Dialogue/BPI_Dialogue.Talk`
  (bind _output_dialogue (break `/Game/Wonderland/System/Dialogue/S_Dialogue` (`|GetArrayItem` (`self.Dialogue`) (`self.TalkIndex`))))
  (`|ExecutionSequence`
    (:`then_0`
      (`Widget.SetVisibility` (`/Game/Wonderland/Prop/Characters/PlayerCharacter/BP_PlayerCharacter.WBPPlayerInfoRef` (`self.BPPlayerCharacterRef`)) "Collapsed")
      (`SceneComponent.SetVisibility` (`self.NPC Interaction Widget`) false false)
      (`/Engine/EditorBlueprintResources/StandardMacros.IncrementInt` (`self.TalkIndex`)
        (:`  `
          (if (< (`self.TalkIndex`) (`KismetArrayLibrary.Array_Length` (`self.Dialogue`)))
            (`self.WBPDialogueRef`
              (:`then`
                _)
              (:`else`
                (bind _returnvalue (`|CreateWidget` "/Game/Wonderland/Widget/GuideCharacter/WBP_Dialogue.WBP_Dialogue_C" (`GameplayStatics.GetPlayerController` 0)))
                (set `self.WBPDialogueRef` _returnvalue)
                (`UserWidget.AddToViewport` (`self.WBPDialogueRef`) 0)))
            (`TextBlock.SetText` (`/Game/Wonderland/Widget/GuideCharacter/WBP_Dialogue.TextBlock_Dialogue` (`self.WBPDialogueRef`)) (`KismetTextLibrary.Conv_StringToText` _output_dialogue))
            (`GameplayStatics.PlaySound2D` "/Game/Wonderland/Sound/SFX/SW_Click.SW_Click" 1.0 1.0 0.0 null null)
            (else
              (`Widget.RemoveFromParent` (`self.WBPDialogueRef`))
              (if (not (`self.IsMyFirstTalk`))
                (set `self.IsMyFirstTalk` true)
                (`UserWidget.AddToViewport` (`/Game/Wonderland/System/Quest/BPC_Quest.WBPQuestType1Ref` (`/Game/Wonderland/Prop/Characters/PlayerCharacter/BP_PlayerCharacter.BPC_Quest` (`self.BPPlayerCharacterRef`))) -1))
              (`Widget.SetVisibility` (`/Game/Wonderland/Prop/Characters/PlayerCharacter/BP_PlayerCharacter.WBPPlayerInfoRef` (`self.BPPlayerCharacterRef`)) "Visible")
              (set `/Game/Wonderland/Prop/Characters/PlayerCharacter/BP_PlayerCharacter.CanTalk` false (`self.BPPlayerCharacterRef`)))))))
    (:`then_1`
      (if (== (`self.TalkIndex`) 8)
        (`Widget.SetVisibility` (`/Game/Wonderland/Widget/GuideCharacter/WBP_Dialogue.TextBlock_NPCName1` (`self.WBPDialogueRef`)) "Hidden")
        (`Widget.SetVisibility` (`/Game/Wonderland/Widget/GuideCharacter/WBP_Dialogue.TextBlock_NPCName2` (`self.WBPDialogueRef`)) "Visible")))))

(fn `UserConstructionScript`)