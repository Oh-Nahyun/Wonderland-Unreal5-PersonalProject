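; Player character Blueprint for Wonderland, handling dialogue, menus, save restoration and game over.
; BeginPlay syncs quest states through the game instance, fills the quest widget from the guide character, loads saved player data and shows unfinished tutorials.
; E talks to overlapping guides via BPI_Dialogue; Tab toggles the quest screen; Escape or U toggles the save menu, both pausing play.
; Death plays a sound, then shows a paused game-over screen.
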(event `self.ReceiveBeginPlay`
  (`KismetSystemLibrary.Delay` 1.0)
  (`|ExecutionSequence`
    (:`then_0`
      (bind _returnvalue (`GameplayStatics.GetActorOfClass` "/Game/Wonderland/Prop/Characters/GuideCharacter/BP_GuideCharacter.BP_GuideCharacter_C"))
      (`/Engine/EditorBlueprintResources/StandardMacros.IsValid` _returnvalue
        (:`Is Valid`
          (set `self.BPGuideCharacterRef` _returnvalue)
          (bind _asbp_game_instance (cast `/Game/Wonderland/GameInstance/BP_GameInstance` (`GameplayStatics.GetGameInstance`)))
          (set `self.BPGameInstanceRef` _asbp_game_instance)
          (`WGameInstanceBase.EnsureAllQuestStatesByDT` (`self.BPGameInstanceRef`) true))))
    (:`then_1`
      (bind _returnvalue_2 (`|CreateWidget` "/Game/Wonderland/Widget/Quest/WBP_MainQuest.WBP_MainQuest_C"))
      (`/Engine/EditorBlueprintResources/StandardMacros.IsValid` _returnvalue_2
        (:`Is Valid`
          (set `self.WBPQuestRef` _returnvalue_2)
          ; 코멘트
          (for _array_element (`/Game/Wonderland/Prop/Characters/GuideCharacter/BP_GuideCharacter.Quests` (`self.BPGuideCharacterRef`))
            (`/Game/Wonderland/Widget/Quest/WBP_MainQuest.CE_AddQuest` (`self.WBPQuestRef`) _array_element)))))
    (:`then_2`
      (`/Engine/EditorBlueprintResources/StandardMacros.IsValid` (`self.PlayerInfoHUD`)
        (:`Is Valid`
          (bind _aswbp_player_info (cast `/Game/Wonderland/Widget/PlayerCharacter/WBP_PlayerInfo` (`self.PlayerInfoHUD`)))
          (set `self.WBPPlayerInfoRef` _aswbp_player_info)
          (`self.CE_LoadPlayer`)
          (`/Game/Wonderland/Widget/PlayerCharacter/WBP_PlayerInfo.CE_PlayAnimFadeOut` (`self.WBPPlayerInfoRef`)))))
    (:`then_3`
      (if (not (`/Game/Wonderland/Widget/PlayerCharacter/WBP_PlayerInfo.IsTutorialEnd` (`self.WBPPlayerInfoRef`)))
        (`KismetSystemLibrary.Delay` 5.0)
        (`Widget.SetVisibility` (`/Game/Wonderland/Widget/PlayerCharacter/WBP_PlayerInfo.WBP_Tutorial` (`self.WBPPlayerInfoRef`)) "HitTestInvisible")
        (`/Game/Wonderland/Widget/Tutorial/WBP_Tutorial.PlayAnim_LeftKey` (`/Game/Wonderland/Widget/PlayerCharacter/WBP_PlayerInfo.WBP_Tutorial` (`self.WBPPlayerInfoRef`)))
        (`/Game/Wonderland/Widget/Tutorial/WBP_Tutorial.PlayAnim_RightKey` (`/Game/Wonderland/Widget/PlayerCharacter/WBP_PlayerInfo.WBP_Tutorial` (`self.WBPPlayerInfoRef`)))))))

(event `Key|E`
  (params (Key :type "Key Structure"))
  (:`Pressed`
    (if (`self.CanTalk`)
      (for _array_element (`self.GetOverlappingActors` "/Game/Wonderland/Prop/Characters/GuideCharacter/BP_GuideCharacter.BP_GuideCharacter_C")
        (set `self.ArrayElement` _array_element)
        (if (`KismetSystemLibrary.DoesImplementInterface` (`self.ArrayElement`) "/Game/Wonderland/System/Dialogue/BPI_Dialogue.BPI_Dialogue_C")
          (message `/Game/Wonderland/System/Dialogue/BPI_Dialogue.Talk` (`self.ArrayElement`)))))))

(event `Key|Tab` :paused true
  (params (Key :type "Key Structure"))
  (:`Pressed`
    (if (not (`self.IsQuestWidgetActive`))
      (`/Game/Wonderland/Widget/PlayerCharacter/WBP_PlayerInfo.CE_PlayAnimFadeIn` (`self.WBPPlayerInfoRef`))
      (`KismetSystemLibrary.Delay` 1.0)
      (`UserWidget.AddToViewport` (`self.WBPQuestRef`) 0)
      (set `self.IsQuestWidgetActive` true)
      (`KismetSystemLibrary.Delay` 1.0)
      (set `PlayerController.bShowMouseCursor` true (`GameplayStatics.GetPlayerController` 0))
      (`WidgetBlueprintLibrary.SetInputMode_GameAndUIEx` (`GameplayStatics.GetPlayerController` 0) (`self.WBPQuestRef`))
      (`GameplayStatics.SetGamePaused` true)
      (else
        (`self.CE_CloseQuest`)))))

(event `CE_CloseQuest`
  (`GameplayStatics.SetGamePaused` false)
  (`/Game/Wonderland/Widget/Quest/WBP_MainQuest.CE_PlayAnimFadeIn` (`self.WBPQuestRef`))
  (`KismetSystemLibrary.Delay` 1.0)
  (`Widget.RemoveFromParent` (`self.WBPQuestRef`))
  (`/Game/Wonderland/Widget/PlayerCharacter/WBP_PlayerInfo.CE_PlayAnimFadeOut` (`self.WBPPlayerInfoRef`))
  (set `self.IsQuestWidgetActive` false)
  (set `PlayerController.bShowMouseCursor` false (`GameplayStatics.GetPlayerController` 0))
  (`WidgetBlueprintLibrary.SetInputMode_GameOnly` (`GameplayStatics.GetPlayerController` 0)))

(event `Key|Escape` :paused true
  (params (Key :type "Key Structure"))
  (:`Pressed`
    (if (`self.IsSaveGameWidgetActive`) :!label _label
      (`GameplayStatics.SetGamePaused` false)
      (`Widget.RemoveFromParent` (`self.WBPSaveGameRef`))
      (set `self.WBPSaveGameRef` null)
      (set `PlayerController.bShowMouseCursor` false (`GameplayStatics.GetPlayerController` 0))
      (`WidgetBlueprintLibrary.SetInputMode_GameOnly` (`GameplayStatics.GetPlayerController` 0))
      (set `self.IsSaveGameWidgetActive` false)
      (else
        (bind _returnvalue (`|CreateWidget` "/Game/Wonderland/Widget/SaveGame/WBP_SaveGame.WBP_SaveGame_C"))
        (set `self.WBPSaveGameRef` _returnvalue)
        (`UserWidget.AddToViewport` (`self.WBPSaveGameRef`) 0)
        (set `PlayerController.bShowMouseCursor` true (`GameplayStatics.GetPlayerController` 0))
        (`WidgetBlueprintLibrary.SetInputMode_GameAndUIEx` (`GameplayStatics.GetPlayerController` 0) (`self.WBPSaveGameRef`))
        (`GameplayStatics.SetGamePaused` true)
        (set `self.IsSaveGameWidgetActive` true)))))

(event `Key|U` :paused true
  (params (Key :type "Key Structure"))
  (:`Pressed`
    (goto _label)))

(event `CE_LoadPlayer`
  (bind _bpsavegameref (`self.BPSaveGameRef`))
  (bind _returnvalue (`GameplayStatics.DoesSaveGameExist` "SaveGameSlot"))
  (bind _asbp_game_instance (cast `/Game/Wonderland/GameInstance/BP_GameInstance` (`GameplayStatics.GetGameInstance`)))
  (if (and _returnvalue (`WGameInstanceBase.bIsGameSaved` _asbp_game_instance))
    (bind _returnvalue_2 (`GameplayStatics.LoadGameFromSlot` "SaveGameSlot"))
    (bind _asbp_save_game (cast `/Game/Wonderland/System/SaveGame/BP_SaveGame` _returnvalue_2))
    (set `self.BPSaveGameRef` _asbp_save_game)
    (`ProgressBar.SetPercent` (`/Game/Wonderland/Widget/PlayerCharacter/WBP_PlayerInfo.ProgressBar_Health` (`self.WBPPlayerInfoRef`)) (`/Game/Wonderland/System/SaveGame/BP_SaveGame.PlayerHealth` (`self.BPSaveGameRef`)))
    (`ProgressBar.SetPercent` (`/Game/Wonderland/Widget/PlayerCharacter/WBP_PlayerInfo.ProgressBar_Stemina` (`self.WBPPlayerInfoRef`)) (`/Game/Wonderland/System/SaveGame/BP_SaveGame.PlayerStemina` (`self.BPSaveGameRef`)))
    (`self.K2_SetActorLocationAndRotation` (`/Game/Wonderland/System/SaveGame/BP_SaveGame.PlayerLocation` _bpsavegameref) (`/Game/Wonderland/System/SaveGame/BP_SaveGame.PlayerRotation` _bpsavegameref))
    (set `WGameInstanceBase.bIsTutorialEnd` (`/Game/Wonderland/System/SaveGame/BP_SaveGame.IsTutorialEnd` (`self.BPSaveGameRef`)) (`self.BPGameInstanceRef`))
    (set `WGameInstanceBase.QuestStates` (`/Game/Wonderland/System/SaveGame/BP_SaveGame.QuestStates` (`self.BPSaveGameRef`)) (`self.BPGameInstanceRef`))
    (else
      (`GameplayStatics.DeleteGameInSlot` "SaveGameSlot"))))

(event `self.SetAfterPlayerDie`
  (`GameplayStatics.PlaySound2D` "/Game/Wonderland/Sound/SFX/SW_GameOver.SW_GameOver" 1.0 1.0 0.0 null null)
  (`KismetSystemLibrary.Delay` 2.5)
  (bind _returnvalue (`|CreateWidget` "/Game/Wonderland/Widget/GameOver/WBP_GameOver.WBP_GameOver_C"))
  (set `self.WBPGameOverRef` _returnvalue)
  (`UserWidget.AddToViewport` (`self.WBPGameOverRef`) 0)
  (`/Game/Wonderland/Widget/GameOver/WBP_GameOver.CE_PlayAnimShowUp` (`self.WBPGameOverRef`))
  (`GameplayStatics.SetGamePaused` true)
  (set `PlayerController.bShowMouseCursor` true (`GameplayStatics.GetPlayerController` 0))
  (`WidgetBlueprintLibrary.SetInputMode_UIOnlyEx` (`GameplayStatics.GetPlayerController` 0) (`self.WBPGameOverRef`)))

(fn `UserConstructionScript`)