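; Door prop that sends the player to MainLevel when they interact while standing near it.
; A sphere overlap toggles the interaction widget, sets an in-range flag and caches the BP_PlayerCharacter reference.
; Tick polls that flag and the player's CanInteraction, then opens the level by name.
; The widget is hidden shortly after BeginPlay, and the overlap flag is set for any actor, before the player cast.
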(event `self.ReceiveBeginPlay`
  (`KismetSystemLibrary.Delay` 0.1)
  (`SceneComponent.SetVisibility` (`self.Door Interaction Widget`) false false))

(event `self.ReceiveTick`
  (params (DeltaSeconds :type "Float (single-precision)"))
  (if (`self.IsInSphereCollision`)
    (`/Engine/EditorBlueprintResources/StandardMacros.IsValid` (`self.BPPlayerCharacterRef`)
      (:`Is Valid`
        (if (`WPlayerCharacter.bCanInteraction` (`self.BPPlayerCharacterRef`))
          (`GameplayStatics.OpenLevel` "MainLevel"))))))

(event `self.SphereCollision.OnComponentBeginOverlap`
  (params (OverlappedComponent :type "PrimitiveComponent Object Reference") (OtherActor :type "Actor Object Reference") (OtherComp :type "PrimitiveComponent Object Reference") (OtherBodyIndex :type Integer) (bFromSweep :type Boolean) (SweepResult :type "HitResult Structure (by ref)"))
  (`SceneComponent.SetVisibility` (`self.Door Interaction Widget`) true false)
  (set `self.IsInSphereCollision` true)
  (bind _asbp_player_character (cast `/Game/Wonderland/Prop/Characters/PlayerCharacter/BP_PlayerCharacter` OtherActor))
  (set `self.BPPlayerCharacterRef` _asbp_player_character))

(event `self.SphereCollision.OnComponentEndOverlap`
  (params (OverlappedComponent :type "PrimitiveComponent Object Reference") (OtherActor :type "Actor Object Reference") (OtherComp :type "PrimitiveComponent Object Reference") (OtherBodyIndex :type Integer))
  (`SceneComponent.SetVisibility` (`self.Door Interaction Widget`) false false)
  (set `self.IsInSphereCollision` false))

(fn `UserConstructionScript`)