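; BP_EnemyController is the AI controller that drives BP_EnemyCharacter through a behavior tree.
; On possess it loads the BP_EnemyBB blackboard, seeds it with the pawn's home location, an idle time and a random navigable target near spawn, then runs BP_EnemyBT1.
; Every tick it copies the character's current enemy state into the blackboard, so the character owns the state that the tree reads.
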(event `self.ReceivePossess`
  (params (PossessedPawn :type "Pawn Object Reference"))
  (bind _asbp_new_enemy_character (cast `/Game/Wonderland/Props/Characters/EnemyCharacter/BP_EnemyCharacter` (`self.K2_GetPawn`)))
  (set `self.EnemyCharacter` _asbp_new_enemy_character)
  (`|ExecutionSequence`
    (:`then_0`
      (`self.UseBlackboard` "/Game/Wonderland/Props/Characters/EnemyCharacter/AI/BP_EnemyBB.BP_EnemyBB"))
    (:`then_1`
      (`BlackboardComponent.SetValueAsVector` (`self.Blackboard`) (`self.HomeLocKey`) (`self.K2_GetActorLocation` (`self.K2_GetPawn`)))
      (`BlackboardComponent.SetValueAsFloat` (`self.Blackboard`) (`self.IdleTimeKey`) 5.0)
      (bind _randomlocation (`NavigationSystemV1.K2_GetRandomLocationInNavigableRadius` (`self.K2_GetActorLocation` (`self.K2_GetPawn`)) 500.0 null null))
      (`BlackboardComponent.SetValueAsVector` (`self.Blackboard`) (`self.TargetLocKey`) _randomlocation))
    (:`then_2`
      (`self.RunBehaviorTree` "/Game/Wonderland/Props/Characters/EnemyCharacter/AI/BP_EnemyBT1.BP_EnemyBT1"))))

(event `self.ReceiveTick`
  (params (DeltaSeconds :type "Float (single-precision)"))
  (`BlackboardComponent.SetValueAsEnum` (`self.Blackboard`) (`self.StateKey`) (`/Game/Wonderland/Props/Characters/EnemyCharacter/BP_EnemyCharacter.CurrentEnemyState` (`self.EnemyCharacter`))))

(fn `UserConstructionScript`)