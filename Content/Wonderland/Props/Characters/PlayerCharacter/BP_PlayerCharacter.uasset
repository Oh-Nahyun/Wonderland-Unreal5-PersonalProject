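; Player character Blueprint that handles talking to the guide, toggling the quest journal and showing the control tutorial.
; On BeginPlay it caches the guide character and, if the player info HUD's tutorial is unfinished, plays its key animations.
; E sends a dialogue interface message to overlapping guides.
; Tab fades the HUD, then opens a UI-only quest widget filled from the guide's quests, or closes it and restores game input.
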(event `self.ReceiveBeginPlay`
  (`KismetSystemLibrary.Delay` 1.0)
  (`|ExecutionSequence`
    (:`then_0`
      (bind _returnvalue (`GameplayStatics.GetActorOfClass` "/Game/Wonderland/Props/Characters/GuideCharacter/BP_GuideCharacter.BP_GuideCharacter_C"))
      (`/Engine/EditorBlueprintResources/StandardMacros.IsValid` _returnvalue
        (:`Is Valid`
          (set `self.BPGuideCharacterRef` _returnvalue))))
    (:`then_1`
      (`/Engine/EditorBlueprintResources/StandardMacros.IsValid` (`self.PlayerInfoHUD`)
        (:`Is Valid`
          (bind _aswbp_player_info (cast `/Game/Wonderland/Widget/PlayerCharacter/WBP_PlayerInfo` (`self.PlayerInfoHUD`)))
          (set `self.WBPPlayerInfoRef` _aswbp_player_info)
          (if (not (`/Game/Wonderland/Widget/PlayerCharacter/WBP_PlayerInfo.IsTutorialEnd` (`self.WBPPlayerInfoRef`)))
            (`KismetSystemLibrary.Delay` 1.0)
            (`Widget.SetVisibility` (`/Game/Wonderland/Widget/PlayerCharacter/WBP_PlayerInfo.WBP_Tutorial` (`self.WBPPlayerInfoRef`)) "HitTestInvisible")
            (`/Game/Wonderland/Widget/Tutorial/WBP_Tutorial.PlayAnim_LeftKey` (`/Game/Wonderland/Widget/PlayerCharacter/WBP_PlayerInfo.WBP_Tutorial` (`self.WBPPlayerInfoRef`)))
            (`/Game/Wonderland/Widget/Tutorial/WBP_Tutorial.PlayAnim_RightKey` (`/Game/Wonderland/Widget/PlayerCharacter/WBP_PlayerInfo.WBP_Tutorial` (`self.WBPPlayerInfoRef`)))))))))

(event `Key|E`
  (params (Key :type "Key Structure"))
  (:`Pressed`
    (for _array_element (`self.GetOverlappingActors` "/Game/Wonderland/Props/Characters/GuideCharacter/BP_GuideCharacter.BP_GuideCharacter_C")
      (set `self.ArrayElement` _array_element)
      (if (`KismetSystemLibrary.DoesImplementInterface` (`self.ArrayElement`) "/Game/Wonderland/Props/Characters/GuideCharacter/BPI_Dialogue.BPI_Dialogue_C")
        (message `/Game/Wonderland/Props/Characters/GuideCharacter/BPI_Dialogue.Talk` (`self.ArrayElement`))))))

(event `Key|Tab`
  (params (Key :type "Key Structure"))
  (:`Pressed`
    (`/Game/Wonderland/Widget/PlayerCharacter/WBP_PlayerInfo.CE_PlayAnimFadeIn` (`self.WBPPlayerInfoRef`))
    (`KismetSystemLibrary.Delay` 1.0)
    (if (not (`self.IsQuestWidgetActive`))
      (`|ExecutionSequence`
        (:`then_0`
          (bind _returnvalue (`|CreateWidget` "/Game/Wonderland/Widget/Quest/WBP_Quest.WBP_Quest_C"))
          (set `self.WBPQuestRef` _returnvalue)
          (`UserWidget.AddToViewport` (`self.WBPQuestRef`) 0)
          (set `self.IsQuestWidgetActive` true))
        (:`then_1`
          (`KismetSystemLibrary.Delay` 1.0)
          (set `PlayerController.bShowMouseCursor` true (`GameplayStatics.GetPlayerController` 0))
          (`WidgetBlueprintLibrary.SetInputMode_UIOnlyEx` (`GameplayStatics.GetPlayerController` 0) (`self.WBPQuestRef`))
          (for _array_element (`/Game/Wonderland/Props/Characters/GuideCharacter/BP_GuideCharacter.Quests` (`self.BPGuideCharacterRef`))
            (`/Game/Wonderland/Widget/Quest/WBP_Quest.CE_AddQuest` (`self.WBPQuestRef`) _array_element))))
      (else
        (`Widget.RemoveFromParent` (`self.WBPQuestRef`))
        (set `self.WBPQuestRef` null)
        (set `PlayerController.bShowMouseCursor` false (`GameplayStatics.GetPlayerController` 0))
        (`WidgetBlueprintLibrary.SetInputMode_GameOnly` (`GameplayStatics.GetPlayerController` 0))
        (set `self.IsQuestWidgetActive` false)))))

(fn `UserConstructionScript`)