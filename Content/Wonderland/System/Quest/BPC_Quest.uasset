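; Quest component that drives the active quest's display and tracks its enemy-elimination objectives.
; On BeginPlay it creates the quest widget and caches the game instance, which holds completion and deactivation states, and the player character, which exposes the main quest menu.
; Eliminated enemies are matched by class, counting down one shared RequiredCount variable.
; At zero it records the objective, then checks quest completion to update both widgets.
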(event `self.ReceiveBeginPlay`
  (bind _returnvalue (`|CreateWidget` "/Game/Wonderland/Widget/Quest/WBP_QuestType1.WBP_QuestType1_C"))
  (set `self.WBPQuestType1Ref` _returnvalue)
  (bind _asbp_game_instance (cast `/Game/Wonderland/GameInstance/BP_GameInstance` (`GameplayStatics.GetGameInstance`)))
  (set `self.BPGameInstanceRef` _asbp_game_instance)
  (bind _asbp_player_character (cast `/Game/Wonderland/Prop/Characters/PlayerCharacter/BP_PlayerCharacter` (`GameplayStatics.GetPlayerCharacter` 0)))
  (set `self.BPPlayerCharacterRef` _asbp_player_character))

(event `CE_SetActiveQuest`
  (bind (_fontobject _fontmaterial _outlinesettings _typefacefontname _size _letterspacing _skewamount _bforcemonospaced _bmaterialisstencil _monospacedwidth) (break `SlateFontInfo` (`TextBlock.Font` (`/Game/Wonderland/Widget/Quest/WBP_QuestType1.TextBlock_Quest` (`self.WBPQuestType1Ref`)))))
  (`TextBlock.SetText` (`/Game/Wonderland/Widget/Quest/WBP_QuestType1.TextBlock_Quest` (`self.WBPQuestType1Ref`)) (`KismetTextLibrary.Conv_StringToText` (`.Name_36_24F5630C4285C72757EB338E602F6241` (break `/Game/Wonderland/System/Quest/S_Quest` (`self.ActiveQuest`)))))
  (`TextBlock.SetFont` (`/Game/Wonderland/Widget/Quest/WBP_QuestType1.TextBlock_Quest` (`self.WBPQuestType1Ref`)) (make `SlateFontInfo` _fontobject _fontmaterial _outlinesettings _typefacefontname 20.0 _letterspacing _skewamount _bforcemonospaced _bmaterialisstencil _monospacedwidth)))

(event `CE_SetQuestObjectives`
  (`/Game/Wonderland/Widget/Quest/WBP_QuestType1.CE_FillQuestObjectives` (`self.WBPQuestType1Ref`) (`self.ActiveQuest`)))

(event `CE_EliminateEnemy`
  (params (EnemyEliminated :type "Actor Object Reference"))
  (bind (_activequest_id _activequest_name _activequest_description _activequest_secundary _activequest_objectives) (break `/Game/Wonderland/System/Quest/S_Quest` (`self.ActiveQuest`)))
  (bind _returnvalue (`KismetStringLibrary.Conv_StringToName` _activequest_id))
  (bind _returnvalue_2 (`WGameInstanceBase.GetStatesById` (`self.BPGameInstanceRef`) _returnvalue))
  (for (_array_element _array_index) _activequest_objectives
    (if (> (`KismetArrayLibrary.Array_Length` _returnvalue_2) 0)
      (bind (_name _actortoeliminate) (break `/Game/Wonderland/System/Quest/S_QuestObjective` _array_element))
      (bind (_targetactorclass _requiredcount _iseliminateenemyobjective) (break `/Game/Wonderland/System/Quest/S_ActorToEliminate` _actortoeliminate))
      (if (and (not (`|GetArrayItem` _returnvalue_2 _array_index)) (== (`GameplayStatics.GetObjectClass` EnemyEliminated) _targetactorclass) _iseliminateenemyobjective)
        (if (not (!= (`self.RequiredCount`) 0))
          (set `self.RequiredCount` _requiredcount))
        (`/Engine/EditorBlueprintResources/StandardMacros.DecrementInt` (`self.RequiredCount`)
          (:`  `
            (`|VariableSetRef` _actortoeliminate (make `/Game/Wonderland/System/Quest/S_ActorToEliminate` _targetactorclass (`self.RequiredCount`) _iseliminateenemyobjective))
            (if (== (`self.RequiredCount`) 0)
              (`WGameInstanceBase.SetObjectiveCompleted` (`self.BPGameInstanceRef`) _returnvalue _array_index true)
              (`/Game/Wonderland/Widget/Quest/WBP_QuestType1.CE_CompleteObjective` (`self.WBPQuestType1Ref`) _returnvalue _name)
              (`self.CE_CheckQuestState` _returnvalue))))))))

(event `CE_CheckQuestState`
  (params (QuestID :type Name))
  (if (`WGameInstanceBase.IsQuestCompletedById` (`self.BPGameInstanceRef`) QuestID)
    (`/Game/Wonderland/Widget/Quest/WBP_QuestType1.CE_ShowCompletedQuest` (`self.WBPQuestType1Ref`))
    (`WGameInstanceBase.ChangeDeactivationState` (`self.BPGameInstanceRef`) QuestID)
    (`/Game/Wonderland/Widget/Quest/WBP_MainQuest.CE_ChangeStateToComplete` (`/Game/Wonderland/Prop/Characters/PlayerCharacter/BP_PlayerCharacter.WBPMainQuestRef` (`self.BPPlayerCharacterRef`)) (`KismetStringLibrary.Conv_NameToString` QuestID))
    (else
      (`/Game/Wonderland/Widget/Quest/WBP_QuestType1.CE_HideCompletedQuest` (`self.WBPQuestType1Ref`)))))

(event `CE_ChangeDeactivationState`
  (params (QuestID :type Name))
  (bind _questdeactivationstates (`WGameInstanceBase.QuestDeactivationStates` (`self.BPGameInstanceRef`)))
  (if (`BlueprintMapLibrary.Map_Contains` _questdeactivationstates QuestID)
    (if (`BlueprintMapLibrary.Map_Find` _questdeactivationstates QuestID)
      (`/Game/Wonderland/Widget/Quest/WBP_QuestSlotType1.CE_DeactivationButtonAndText` (`/Game/Wonderland/Widget/Quest/WBP_MainQuest.WBPQuestSlotType1Ref` (`/Game/Wonderland/Prop/Characters/PlayerCharacter/BP_PlayerCharacter.WBPMainQuestRef` (`self.BPPlayerCharacterRef`))))
      (`/Game/Wonderland/Widget/Quest/WBP_QuestType1.CE_HideCompletedQuest` (`self.WBPQuestType1Ref`))
      (else
        (`/Game/Wonderland/Widget/Quest/WBP_QuestSlotType1.CE_ActivationButtonAndText` (`/Game/Wonderland/Widget/Quest/WBP_MainQuest.WBPQuestSlotType1Ref` (`/Game/Wonderland/Prop/Characters/PlayerCharacter/BP_PlayerCharacter.WBPMainQuestRef` (`self.BPPlayerCharacterRef`))))
        (`/Game/Wonderland/Widget/Quest/WBP_QuestType1.CE_ShowCompletedQuest` (`self.WBPQuestType1Ref`))))))